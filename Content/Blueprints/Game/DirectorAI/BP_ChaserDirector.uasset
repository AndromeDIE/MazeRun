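; AI director for maze chasers that paces pressure on the player via a tension level driven by active chases.
; It registers all BPI_Chaser actors, updates and evaluates tension each tick, and feeds a debug meter.
; Reaching the threshold triggers a timed scatter and reset, while prolonged zero tension sends a random chaser near the player with a warning.
; Cleared maze zones send every chaser to random zone corners.
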(event Custom|Event%20StartScatter
  (Utilities|FlowControl|DoOnce false
    (:Completed
      (Scatter|ToggleScatterforAllChasers true)
      (Utilities|Time|SetTimerbyEvent (delegate Custom|Event%20EndScatter) 1e+01))))

(event Custom|Event%20ResetTension
  (Variables|TensionMeter|SetCurrentTensionLevel 0.0))

(event Custom|Event%20OnChaserDetectedTarget
  (bind _result (Math|Integer|IncrementInt (Variables|Default|GetActiveChases))
    (:%20%20
      (Development|PrintText (Utilities|Text|FormatText "Chaser Mode Toggled. Active Chases: {Amount}" _result))
      (Utilities|Time|ClearandInvalidateTimerbyHandle (stale Custom|Event%20OnChaserLostTarget _returnvalue)))))

(event Custom|Event%20OnChaserLostTarget
  (bind _result (Math|Integer|DecrementInt (Variables|Default|GetActiveChases))
    (:%20%20
      (Development|PrintText (Utilities|Text|FormatText "Chaser Mode Toggled. Active Chases: {Amount}" _result))
      (if (== _result 0)
        (bind _returnvalue (Utilities|Time|SetTimerbyEvent (EventDispatchers|CreateEvent :!event Custom|Event%20ResetTension) (Variables|TensionMeter|GetTensionResetTime)))))))

(event Custom|Event%20EndScatter
  (CallFunction|EventResetTension)
  (Scatter|ToggleScatterforAllChasers false)
  (Utilities|FlowControl|DoOnce false) ; enters at Reset
)

(event Custom|Event%20OnZoneCleared
  (params (ZoneCornerLocations :type Array%20of%20Vectors))
  (Command|CommandAllChaserstoRandomLocationfromArray ZoneCornerLocations))

(event Custom|Event%20OnTensionReachedZero
  (Utilities|FlowControl|DoOnce false
    (:Completed
      (bind _returnvalue (Utilities|Time|SetTimerbyEvent (delegate Custom|Event%20OnProlongedTensionlessness) 2e+01)))))

(event Custom|Event%20OnProlongedTensionlessness
  (Command|CommandRandomChasertoPlayerProximity)
  (Utilities|FlowControl|DoOnce false) ; enters at Reset
)

(event Custom|Event%20OnTensionIsNotZero
  (Utilities|Time|ClearandInvalidateTimerbyHandle (stale Custom|Event%20OnTensionReachedZero _returnvalue))
  (Utilities|FlowControl|DoOnce false) ; enters at Reset
)

(event EventBeginPlay
  (Utilities|FlowControl|DelayUntilNextTick)
  (Setup|GetAllChasers)
  (Debug|DoDebugThings)
  (Setup|SetupZoneClearEvent)
  (Setup|GetPlayerReference)
  (Utilities|FlowControl|DelayUntilNextTick)
  (Actor|Tick|SetActorTickEnabled true))

(event EventTick
  (params (DeltaSeconds :type Float%20%28single-precision%29))
  (Tension|HandleTension DeltaSeconds))

(fn ConstructionScript)

(fn GetAllChasers
  (bind _outactors (Actor|GetAllActorswithInterface "/Game/Blueprints/Enemy/BPI_Chaser.BPI_Chaser_C"))
  (for _array_element _outactors
    (bind _asbpi_chaser (Utilities|Casting|CastToBPI_Chaser _array_element))
    (Utilities|Array|Add (Variables|Default|GetChasers) _asbpi_chaser)
    (Default|RegistertoChaserDirector _asbpi_chaser self))
  (Development|PrintText (Utilities|Text|FormatText "Chasers in Level: {Amount}" (Utilities|Array|Length (Variables|Default|GetChasers)))))

(fn DoDebugThings
  (Setup|InitializeTensionMeterWidget))

(fn InitializeTensionMeterWidget
  (bind _returnvalue (UserInterface|CreateWidget "/Game/UI/Debug/WBP_TensionMeter.WBP_TensionMeter_C"))
  (bind _output_get (Variables|TensionMeter|SetTensionMeterRef _returnvalue))
  (UserInterface|Viewport|AddtoViewport _output_get 0)
  (Default|EventSetup _output_get (Variables|TensionMeter|GetTensionThreshold)))

(fn EvaluateTensionLevel
  (params (NewTensionLevel :type Float%20%28double-precision%29))
  (Utilities|FlowControl|Sequence
    (:then_0
      ;[0.364 0.381 1] Check if Tension Threshold was reached
      (if (>= NewTensionLevel (Variables|TensionMeter|GetTensionThreshold))
        (Tension|OnTensionThresholdReached)))
    (:then_1
      (if (== NewTensionLevel 0.0)
        (CallFunction|EventonTensionReachedZero)
        (else
          (CallFunction|EventonTensionIsNotZero))))))

(fn SetupZoneClearEvent
  (bind _outactors (Actor|GetAllActorsOfClass "/Game/Blueprints/Zones/BP_MazeZone.BP_MazeZone_C"))
  (for _array_element _outactors
    (EventDispatchers|BindEventtoZoneCleared _array_element (EventDispatchers|CreateEvent :!event Custom|Event%20OnZoneCleared))))

(fn CommandAllChaserstoRandomLocationfromArray
  (params (Corners :type Array%20of%20Vectors))
  (for _array_element (Variables|Default|GetChasers)
    (Command|CommandChasertoLocation _array_element (Utilities|Array|Get(acopy) Corners (Math|Random|RandomInteger (Utilities|Array|Length Corners))))))

(fn CommandChasertoLocation
  (params (ChaserToCommand :type BPI%20Chaser%20Interface) (CommandLocation :type Vector))
  (Default|CommandtoLocation ChaserToCommand CommandLocation))

(fn HandleTension
  (params (Delta :type Float%20%28double-precision%29))
  (bind _output_get (Variables|TensionMeter|SetCurrentTensionLevel (|CalculateNewTensionLevel Delta)))
  (Tension|EvaluateTensionLevel _output_get)
  (Tension|UpdateTensionUI _output_get)
  (Development|PrintString (Utilities|String|ToString(Float) _output_get) true true "(R=0.843561,G=0.000000,B=1.000000,A=1.000000)" 0.1 "Tension"))

(fn UpdateTensionUI
  (params (CurrentTension :type Float%20%28double-precision%29))
  (bind _tensionmeterref (Variables|TensionMeter|GetTensionMeterRef)
    (:then
      (Default|EventUpdateTensionMeter _tensionmeterref CurrentTension))
    (:else)))

(fn OnTensionThresholdReached
  (CallFunction|EventStartScatter)
  (CallFunction|EventResetTension))

(fn ToggleScatterforAllChasers
  (params (Active? :type Boolean))
  (for _array_element (Variables|Default|GetChasers)
    (Default|ToggleScatter _array_element Active?)))

(fn CommandRandomChasertoPlayerProximity
  (bind _randomlocation (CallFunction|GetRandomLocationClosetoPlayer))
  (bind _outrandomchaser (CallFunction|GetRandomChaser))
  (Command|CommandChasertoLocation _outrandomchaser _randomlocation)
  (Audio|PlaySoundatLocation (Variables|Default|GetSFX_LowTensionGhostCommand) _randomlocation "0, 0, 0" 1.0 1.0 0.0 0 0 0 0)
  (bind _returnvalue (UserInterface|CreateWidget "/Game/UI/GamePrompts/WBP_BasePrompt.WBP_BasePrompt_C"))
  (UserInterface|Viewport|AddtoViewport _returnvalue 0)
  (Default|EventShowPrompt _returnvalue "An enemy is approaching! Stay out of sight!" 45.0))

(fn GetRandomChaser
  (LocalVariables|SetRandomIndex (Math|Random|RandomInteger (Utilities|Array|Length (Variables|Default|GetChasers))))
  (for (_array_element _array_index) (Variables|Default|GetChasers)
    (if (== _array_index (LocalVariables|GetRandomIndex))
      (return _array_element))))

(fn GetPlayerReference
  (bind _returnvalue (Actor|GetActorOfClass "/Game/Blueprints/Player/BP_Player.BP_Player_C"))
  (Variables|Default|SetPlayerRef _returnvalue))

(fn GetRandomLocationClosetoPlayer
  (bind _randomlocation (Class|NavigationSystemV1|GetRandomLocationinNavigableRadius (Transformation|GetActorLocation (Variables|Default|GetPlayerRef)) 5e+02 0 0))
  (return _randomlocation))