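; Game mode that spawns enemies from a data table and starts a chaser director once all of them are in play.
; Each table row gives the enemy class, spawn location and tag of the zone corner used as its scatter target.
; BeginPlay sets a countdown from the row count, which each enemy's spawned event decrements.
; At zero it spawns BP_ChaserDirector and binds an event to the pickup manager's half-orbs-collected notification.
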(event Custom|Event%20AllEnemiesSpawned
  (CallFunction|InitializeChaserDirector))

(event Custom|Event%20OnEnemySpawned
  (bind _result (Math|Integer|DecrementInt (Variables|Default|GetEnemyAmount))
    (:%20%20
      (if (== _result 0)
        (CallFunction|EventAllEnemiesSpawned)))))

(event EventBeginPlay
  (CallFunction|InitializeEnemyAmount)
  (|CallParentFunction))

(fn ConstructionScript)

(fn InitializeChaserDirector
  (bind _returnvalue (Game|SpawnActorfromClass "/Game/Blueprints/Game/DirectorAI/BP_ChaserDirector.BP_ChaserDirector_C" (Math|Transform|MakeTransform "0, 0, 0" "0, 0, 0" "1.000000,1.000000,1.000000") "Undefined" "MultiplyWithRoot" 0 0))
  (bind _output_get (Variables|Default|SetChaserDirectorRef _returnvalue))
  (EventDispatchers|BindEventtoHalfOrbsCollected (Variables|Default|GetPickupManagerRef) (EventDispatchers|CreateEvent _output_get :!event EventonHalfOrbsCollected)))

(fn VirtualInitializeEnemies
  (bind _outrownames (DataTable|GetDataTableRowNames "/Game/Blueprints/Game/DirectorAI/DT_DirectorGameModeSpawnInfo.DT_DirectorGameModeSpawnInfo"))
  (for _array_element _outrownames
    (bind _returnvalue (Utilities|GetDataTableRow "/Game/Blueprints/Game/DirectorAI/DT_DirectorGameModeSpawnInfo.DT_DirectorGameModeSpawnInfo" _array_element)
      (:then
        (bind _returnvalue_2 (Game|SpawnActorfromClass (.EnemyToSpawn (Utilities|Struct|BreakS_GameModeSpawnInfo _returnvalue)) (Math|Transform|MakeTransform (.SpawnLocation (Utilities|Struct|BreakS_GameModeSpawnInfo _returnvalue)) "0, 0, 0" "1.000000,1.000000,1.000000") "Undefined" "MultiplyWithRoot" 0 0))
        (EventDispatchers|BindEventtoSpawned _returnvalue_2 (EventDispatchers|CreateEvent :!event Custom|Event%20OnEnemySpawned))
        (bind _outactors (Actor|GetAllActorsOfClasswithTag "/Game/Blueprints/Zones/BP_ZoneCorner.BP_ZoneCorner_C" (.CornerTag (Utilities|Struct|BreakS_GameModeSpawnInfo _returnvalue))))
        (Variables|/Game/Blueprints/Enemy/DirectorControlled/BP_EnemyBase.BP_EnemyBase_C|SetScatterCorner _returnvalue_2 (Utilities|Array|Get(acopy) _outactors))
        (Default|SetNewScatterLocation _returnvalue_2)))))

(fn InitializeEnemyAmount
  (bind _outrownames (DataTable|GetDataTableRowNames "/Game/Blueprints/Game/DirectorAI/DT_DirectorGameModeSpawnInfo.DT_DirectorGameModeSpawnInfo"))
  (Variables|Default|SetEnemyAmount (Utilities|Array|Length _outrownames)))