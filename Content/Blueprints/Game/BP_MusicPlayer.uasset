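; Music player actor that crossfades between tense background music and a chase track as the player is spotted or forgotten.
; On BeginPlay it binds to spotted and forgotten events on either the chaser director or an individual chase AI controller, based on the game instance's mode.
; Tension start cancels any pending stop timer, while stopping is timer-delayed.
; Track swaps fade out, change sound and fade in.
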(event Custom|Event%20StartTension
  (bind _fadeduration (Variables|Default|GetFadeDuration))
  (bind _audiocomponent (Variables|Components|GetAudioComponent))
  (Utilities|Time|ClearandInvalidateTimerbyHandle (stale Custom|Event%20StopTensionTimerStart _returnvalue))
  (if (not (Variables|Default|GetIsTension?))
    (Variables|Default|SetIsTension? true)
    (Audio|Components|Audio|FadeOut (Variables|Components|GetAudioComponent) _fadeduration 0.0 "Linear" :!class /Script/Engine.AudioComponent)
    (Utilities|FlowControl|Delay _fadeduration)
    (Audio|Components|Audio|SetSound _audiocomponent "/Game/Audio/BGM/knock-knock-horror-creepy-scary-thriller-trailer-teaser-177239.knock-knock-horror-creepy-scary-thriller-trailer-teaser-177239")
    (Audio|Components|Audio|Play _audiocomponent 15.0)
    (Audio|Components|Audio|FadeIn _audiocomponent (Variables|Default|GetFadeDuration) 1.0 0.0 "Linear" :!class /Script/Engine.AudioComponent)))

(event Custom|Event%20StopTensionTimerStart
  (bind _returnvalue (Utilities|Time|SetTimerbyEvent (delegate Custom|Event%20StopTension) (Variables|Default|GetFadeDuration))))

(event Custom|Event%20StopTension
  (bind _fadeduration (Variables|Default|GetFadeDuration))
  (bind _audiocomponent (Variables|Components|GetAudioComponent))
  (Audio|Components|Audio|FadeOut (Variables|Components|GetAudioComponent) _fadeduration 0.0 "Linear" :!class /Script/Engine.AudioComponent)
  (Utilities|FlowControl|Delay _fadeduration)
  (Audio|Components|Audio|SetSound _audiocomponent "/Game/Audio/BGM/tense-horror-background-174809.tense-horror-background-174809")
  (Audio|Components|Audio|Play _audiocomponent 1e+01)
  (Audio|Components|Audio|FadeIn _audiocomponent (Variables|Default|GetFadeDuration) 1.0 0.0 "Linear" :!class /Script/Engine.AudioComponent)
  (Variables|Default|SetIsTension? false))

(event EventBeginPlay
  (Utilities|FlowControl|DelayUntilNextTick)
  (bind _out_gamemode (Class|IGame|GetGameMode(Message) (Game|GetGameInstance)))
  (switch Utilities|FlowControl|Switch|SwitchonE_GameMode _out_gamemode
    (:NewEnumerator0
      (bind _returnvalue (Actor|GetActorOfClass "/Game/Blueprints/Game/DirectorAI/BP_ChaserDirector.BP_ChaserDirector_C"))
      (EventDispatchers|BindEventtoPlayerSpotted _returnvalue (EventDispatchers|CreateEvent :!event Custom|Event%20StartTension))
      (EventDispatchers|BindEventtoPlayerForgotten _returnvalue (EventDispatchers|CreateEvent :!event Custom|Event%20StopTensionTimerStart)))
    (:NewEnumerator1
      (bind _returnvalue_2 (Actor|GetActorOfClass "/Game/Blueprints/Enemy/Individual/AIC_IndividualChaseController.AIC_IndividualChaseController_C"))
      (EventDispatchers|BindEventtoPlayerSpotted _returnvalue_2 (EventDispatchers|CreateEvent :!event Custom|Event%20StartTension))
      (EventDispatchers|BindEventtoPlayerForgotten _returnvalue_2 (EventDispatchers|CreateEvent :!event Custom|Event%20StopTensionTimerStart))))
  (CallFunction|EventStopTension))

(event EventTick
  (params (DeltaSeconds :type Float%20%28single-precision%29)))

(fn ConstructionScript)