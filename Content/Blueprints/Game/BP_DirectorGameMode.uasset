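; Game mode that directs an orb-collecting chase game, handling startup, win and lose outcomes, pausing and quitting.
; On BeginPlay it spawns pickup, chaser and minimap managers, binds orb-completion and player-death events, and shows an objective prompt.
; Winning pauses behind a game-over screen, whereas losing opens FirstPersonMap.
; A lazily created pause menu toggles input mode, a debug event toggles chaser scatter through BPI_Chaser, and GetDifficulty returns a fixed value.
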(event EventBeginPlay
  (Setup|InitializePickupManager)
  (Setup|InitializeLoseCondition)
  (Setup|InitializeChaseDirector)
  (Setup|InitializeMinimapManager)
  (CallFunction|ShowStarterPrompt))

(event EventLoseGame
  (Game|OpenLevel(byObjectReference) "/Game/Levels/FirstPersonMap/FirstPersonMap.FirstPersonMap"))

(event EventWinGame
  (bind _returnvalue (UserInterface|CreateWidget "/Game/UI/GameOverWidgets/WBP_GameOverScreen.WBP_GameOverScreen_C"))
  (UserInterface|Viewport|AddtoViewport _returnvalue 0)
  (Game|SetGamePaused true))

(event EventDebugScatter
  (bind _isa (Utilities|FlowControl|FlipFlop)
    (:A
      _)
    (:B
      _))
  (bind _outactors (Actor|GetAllActorswithInterface "/Game/Blueprints/Enemy/BPI_Chaser.BPI_Chaser_C"))
  (for _array_element _outactors
    (Class|BPIChaser|ToggleScatter(Message) _array_element _isa)))

(event EventQuitGame
  (Game|QuitGame 0 "Quit" false))

(event EventTogglePauseGame
  (Variables|Default|GetPauseMenuRef
    (:then
      _)
    (:else
      (CallFunction|SetupPauseMenu)))
  (bind _isa (Utilities|FlowControl|FlipFlop)
    (:A
      _)
    (:B
      _))
  (CallFunction|HandlePauseState _isa))

(fn ConstructionScript)

(fn InitializePickupManager
  (bind _returnvalue (Game|SpawnActorfromClass "/Game/Blueprints/Game/BP_PickupManager.BP_PickupManager_C" (Math|Transform|MakeTransform "0, 0, 0" "0, 0, 0" "1.000000,1.000000,1.000000") "Undefined" "MultiplyWithRoot" 0 0))
  (bind _output_get (Variables|Default|SetPickupManagerRef _returnvalue))
  (EventDispatchers|BindEventtoAllOrbsCollected _output_get (EventDispatchers|CreateEvent :!event WinGame)))

(fn InitializeLoseCondition
  (bind _returnvalue (Actor|GetActorOfClass "/Game/Blueprints/Player/BP_Player.BP_Player_C"))
  (Utilities|IsValid _returnvalue
    (:Is%20Valid
      (EventDispatchers|BindEventtoDied _returnvalue (EventDispatchers|CreateEvent :!event LoseGame)))))

(fn InitializeChaseDirector
  (bind _returnvalue (Game|SpawnActorfromClass "/Game/Blueprints/Game/DirectorAI/BP_ChaserDirector.BP_ChaserDirector_C" (Math|Transform|MakeTransform "0, 0, 0" "0, 0, 0" "1.000000,1.000000,1.000000") "Undefined" "MultiplyWithRoot" 0 0))
  (Variables|Default|SetChaserDirectorRef _returnvalue))

(fn InitializeMinimapManager
  (bind _returnvalue (Game|SpawnActorfromClass "/Game/Blueprints/Game/BP_MinimapManager.BP_MinimapManager_C" (Math|Transform|MakeTransform "0, 0, 0" "0, 0, 0" "1.000000,1.000000,1.000000") "Undefined" "MultiplyWithRoot" 0 0))
  (Variables|Default|SetMinimapManagerRef _returnvalue))

(fn ShowStarterPrompt
  (bind _returnvalue (UserInterface|CreateWidget "/Game/UI/GamePrompts/WBP_BasePrompt.WBP_BasePrompt_C"))
  (UserInterface|Viewport|AddtoViewport _returnvalue 0)
  (Default|EventShowPrompt :self _returnvalue :FontSize 9e+01 :TextToShow "Collect all blue orbs!")
  (EventDispatchers|BindEventtoAnimationFinished _returnvalue (EventDispatchers|CreateEvent :!event ShowControls)))

(fn ShowControls
  (bind _returnvalue (UserInterface|CreateWidget "/Game/UI/Player_HUD/WBP_Controls.WBP_Controls_C"))
  (UserInterface|Viewport|AddtoViewport _returnvalue 0))

(fn SetupPauseMenu
  (bind _returnvalue (UserInterface|CreateWidget "/Game/UI/Menu/WBP_PauseMenu.WBP_PauseMenu_C"))
  (bind _output_get (Variables|Default|SetPauseMenuRef _returnvalue))
  (UserInterface|Viewport|AddtoViewport _output_get 0)
  (EventDispatchers|BindEventtoResumeButtonClicked _output_get (EventDispatchers|CreateEvent :!event TogglePauseGame))
  (EventDispatchers|BindEventtoQuitButtonClicked _output_get (EventDispatchers|CreateEvent :!event QuitGame)))

(fn HandlePauseState
  (params (Paused? :type Boolean))
  (bind _returnvalue (Game|GetPlayerController 0))
  (bind _returnvalue_2 (Game|GetPlayerController 0))
  (Widget|SetVisibility (Variables|Default|GetPauseMenuRef) (select Paused? "Visible" "Hidden"))
  (Game|SetGamePaused Paused?)
  (if Paused?
    (Input|SetInputModeGameandUI _returnvalue_2 (Variables|Default|GetPauseMenuRef) "DoNotLock" false false)
    (Variables|/Script/Engine.PlayerController|SetbShowMouseCursor _returnvalue_2 true)
    (else
      (Input|SetInputModeGameOnly _returnvalue false)
      (Variables|/Script/Engine.PlayerController|SetbShowMouseCursor _returnvalue false))))

(fn GetDifficulty
  (return "NewEnumerator0"))