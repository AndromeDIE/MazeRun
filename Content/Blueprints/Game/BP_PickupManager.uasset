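; BP_PickupManager tracks collection of the target orbs in the level and signals when all have been picked up.
; On BeginPlay it counts every BP_TargetOrb as the maximum and binds an event to each orb's PickedUp dispatcher.
; TargetOrbWasPickedUp increments a counter and calls the AllOrbsCollected dispatcher when the count equals that maximum.
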(event Custom|Event%20TargetOrbWasPickedUp
  (bind _result (Math|Integer|IncrementInt (Variables|Default|GetPickedUpOrbs))
    (:%20%20
      (if (== _result (Variables|Default|GetMaxOrbs))
        (Default|CallAllOrbsCollected)))))

(event EventBeginPlay
  (CallFunction|SetupTargetOrbCount))

(fn ConstructionScript)

(fn SetupTargetOrbCount
  (bind _outactors (Actor|GetAllActorsOfClass "/Game/Blueprints/GameObjects/Pickups/BP_TargetOrb.BP_TargetOrb_C"))
  (Variables|Default|SetMaxOrbs (Utilities|Array|Length _outactors))
  (for _array_element _outactors
    (EventDispatchers|BindEventtoPickedUp _array_element (EventDispatchers|CreateEvent :!event Custom|Event%20TargetOrbWasPickedUp))))