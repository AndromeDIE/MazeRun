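; A trigger zone that recolours the point lights inside it once every target orb in the zone is picked up.
; One tick after BeginPlay it gathers PointLights located within the actor's bounds and counts BP_TargetOrbs overlapping TriggerZone, binding to their pickup events.
; Each pickup decrements the count; at zero, it sets all gathered lights to the completion colour and prints a message.
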(event Custom|Event%20OnTargetOrbInZonePickedUp
  (params (PickupLocation :type Vector))
  (bind _result (Math|Integer|DecrementInt (Variables|Default|GetTargetOrbsInZone))
    (:%20%20
      (if (== _result 0)
        (CallFunction|EventAllTargetOrbsinZonePickedUp)))))

(event Custom|Event%20AllTargetOrbsInZonePickedUp
  (for _array_element (Variables|Default|GetLightsInZone)
    (Rendering|Components|Light|SetLightColor (Variables|/Script/Engine.PointLight|GetPointLightComponent _array_element) (Variables|Default|GetColorChangeOnZoneCompletion) true))
  (Development|PrintString "All orbs collected"))

(event EventBeginPlay
  (Utilities|FlowControl|DelayUntilNextTick)
  (CallFunction|GetLightsinTriggerZone)
  (CallFunction|RegisterTargetOrbsinZone))

(fn ConstructionScript)

(fn GetLightsinTriggerZone
  (bind (_origin _boxextent) (Collision|GetActorBounds false false))
  (bind _outactors (Actor|GetAllActorsOfClass "/Script/Engine.PointLight"))
  (for _array_element _outactors
    (if (Math|Geometry|IsPointinBox (Transformation|GetActorLocation _array_element) _origin _boxextent)
      (Utilities|Array|Add (Variables|Default|GetLightsInZone) _array_element)))
  (Development|PrintString (Utilities|String|ToString(Integer) (Utilities|Array|Length (Variables|Default|GetLightsInZone)))))

(fn RegisterTargetOrbsinZone
  (bind _triggerzone (Variables|Default|GetTriggerZone))
  (bind _overlappingactors (Collision|GetOverlappingActors _triggerzone "/Game/Blueprints/GameObjects/Pickups/BP_TargetOrb.BP_TargetOrb_C" :!class /Script/Engine.PrimitiveComponent))
  (Variables|Default|SetTargetOrbsInZone (Utilities|Array|Length _overlappingactors))
  (for _array_element _overlappingactors
    (bind _asbp_target_orb (Utilities|Casting|CastToBP_TargetOrb _array_element))
    (EventDispatchers|BindEventtoPickedUp _asbp_target_orb (EventDispatchers|CreateEvent :!event Custom|Event%20OnTargetOrbInZonePickedUp))))