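; Blueprint function library that maps chaser blackboard key enums to their blackboard key names.
; GetChaserBBKey covers the full chaser key set: target, scatter, current mode, and normal and high-priority command locations.
; GetIndividualChaserBBKey covers a smaller set of only target actor and target location.
; Both are plain switch lookups, keeping key name strings in one place.
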(fn GetChaserBBKey
  (params (DesiredBBKey :type E_ChaserBBKey%20Enum :default "NewEnumerator0"))
  (switch Utilities|FlowControl|Switch|SwitchonE_ChaserBBKey DesiredBBKey
    (:NewEnumerator0
      (return "TargetActor"))
    (:NewEnumerator1
      (return "TargetLocation"))
    (:NewEnumerator2
      (return "IsScattering"))
    (:NewEnumerator3
      (return "ScatterLocation"))
    (:NewEnumerator4
      (return "CurrentChaserMode"))
    (:NewEnumerator5
      (return "CommandLocation"))
    (:NewEnumerator6
      (return "HighPrioCommandLocation"))))

(fn GetIndividualChaserBBKey
  (params (Desired%20BB%20Key :type E_IndividualChaserBBKey%20Enum :default "NewEnumerator0"))
  (switch Utilities|FlowControl|Switch|SwitchonE_IndividualChaserBBKey Desired%20BB%20Key
    (:NewEnumerator0
      (return "TargetActor"))
    (:NewEnumerator1
      (return "TargetLocation"))))