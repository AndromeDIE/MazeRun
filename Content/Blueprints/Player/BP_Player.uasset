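; First-person player Blueprint that adds leaning, crouching, item pickup, interaction and death handling.
; Leaning rolls a camera pivot with an eased move while pawn control rotation is off; crouching resizes the capsule.
; Overlaps auto-collect pickupable, non-interactable actors through interfaces, while the interact input messages the first overlapping interactable.
; A debug key toggles god mode, which blocks death and removes the Player tag.
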(event Input|EnhancedActionEvents|EnhancedInputActionIA_Lean
  (params (ActionValue :type Float%20%28double-precision%29) (ElapsedSeconds :type Float%20%28double-precision%29) (TriggeredSeconds :type Float%20%28double-precision%29) (InputAction :type Input%20Action%20Object%20Reference :default "/Game/Input/Actions/IA_Lean.IA_Lean"))
  (:Started
    (|TryLeanInDirection ActionValue))
  (:Completed
    (|ResetLean)))

(event Input|EnhancedActionEvents|EnhancedInputActionIA_Crouch
  (params (ActionValue :type Boolean) (ElapsedSeconds :type Float%20%28double-precision%29) (TriggeredSeconds :type Float%20%28double-precision%29) (InputAction :type Input%20Action%20Object%20Reference :default "/Game/Input/Actions/IA_Crouch.IA_Crouch"))
  (:Started
    (CallFunction|CustomCrouch))
  (:Completed
    (CallFunction|CustomUnCrouch)))

(event Input|EnhancedActionEvents|EnhancedInputActionIA_Interact
  (params (ActionValue :type Boolean) (ElapsedSeconds :type Float%20%28double-precision%29) (TriggeredSeconds :type Float%20%28double-precision%29) (InputAction :type Input%20Action%20Object%20Reference :default "/Game/Input/Actions/IA_Interact.IA_Interact"))
  (CallFunction|TryInteractwithNearbyInteractable))

(event EventDie
  (if (not (Variables|Default|GetIsGodMode))
    (Default|CallDied)))

(event Collision|EventActorBeginOverlap
  (params (OtherActor :type Actor%20Object%20Reference))
  (CallFunction|TryPickupItem OtherActor))

(event Input|KeyboardEvents|DebugKeyI
  (params (Key :type Key%20Structure :default "None") (ActionValue :type Input%20Action%20Value%20Structure))
  (bind _tags (Variables|Actor|GetTags))
  (:Pressed
    (bind _isa (Utilities|FlowControl|FlipFlop)
      (:A
        _)
      (:B
        _))
    (bind _output_get (Variables|Default|SetIsGodMode _isa))
    (Development|PrintText (Utilities|Text|FormatText "IsGodMode: {Value}" _output_get))
    (if _isa
      (Utilities|Array|RemoveItem _tags "Player")
      (else
        (Utilities|Array|Add _tags "Player")))))

(fn ConstructionScript)

(fn DisableCameraPawnControl
  (Variables|/Script/Engine.CameraComponent|SetbUsePawnControlRotation (Variables|Default|GetFirstPersonCamera) false))

(fn EnableCameraPawnControl
  (Variables|/Script/Engine.CameraComponent|SetbUsePawnControlRotation (Variables|Default|GetFirstPersonCamera) true))

(fn CustomCrouch
  (Components|Capsule|SetCapsuleHalfHeight (Variables|Collision|GetCapsuleComponent) (LocalVariables|GetCrouchHeight) true)
  (Variables|Default|SetIsCrouching true))

(fn CustomUnCrouch
  (Components|Capsule|SetCapsuleHalfHeight (Variables|Collision|GetCapsuleComponent) (LocalVariables|GetStandHeight) true)
  (Variables|Default|SetIsCrouching false))

(fn TryPickupItem
  (params (OverlappedActor :type Actor%20Object%20Reference))
  (if (and (Utilities|DoesObjectImplementInterface OverlappedActor "/Game/Blueprints/Interfaces/I_Pickupable.I_Pickupable_C") (not (Utilities|DoesObjectImplementInterface OverlappedActor "/Game/Blueprints/Interfaces/I_Interactable.I_Interactable_C")))
    (Class|IPickupable|PickUp(Message) OverlappedActor)))

(fn TryInteractwithNearbyInteractable
  (bind _array_element (Utilities|Array|ForEachLoopwithBreak (Collision|GetOverlappingActors 0 :!class /Script/Engine.Actor) :!label _label)
    (:LoopBody
      (if (Utilities|DoesObjectImplementInterface _array_element "/Game/Blueprints/Interfaces/I_Interactable.I_Interactable_C")
        (Class|IInteractable|Interact(Message) _array_element)
        (goto _label Break)))))