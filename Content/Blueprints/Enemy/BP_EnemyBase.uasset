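; Base Blueprint for chaser enemies (ghosts) that patrol, chase, scatter and kill I_Killable actors through an overlap kill zone.
; Chase mode changes, mainly from behavior tree services, toggle the kill zone and walk speed.
; Paired DoOnce gates keep target detected/lost dispatches balanced for the Chaser Director's active chase count.
; Director commands write move locations by priority or scatter state to the Blackboard, with scatter clearing the current target.
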(event OnComponentBeginOverlap(KillZone)
  (params (OverlappedComponent :type Primitive%20Component%20Object%20Reference) (OtherActor :type Actor%20Object%20Reference) (OtherComp :type Primitive%20Component%20Object%20Reference) (OtherBodyIndex :type Integer) (bFromSweep :type Boolean) (SweepResult :type Hit%20Result%20Structure%20%28by%20ref%29))
  ;[0.2275 0.2275 0.2275] Simple KillSphere
  (CallFunction|TryKillNearby OtherActor))

(event EventRegistertoChaserDirector
  (params (ChaserDirectorInQuestion :type BP%20Chaser%20Director%20Object%20Reference))
  ;[0.2275 0.2275 0.2275] Register to Chaser Director via Event Dispatch Binds
  (CallFunction|BindtoChaserDirector ChaserDirectorInQuestion))

(event EventNotifyTargetDetected
  ;[0.2275 0.2275 0.2275] Called when Chaser Mode changes. Do Once Gates to keep the ActiveChase counter in check
  (Utilities|FlowControl|DoOnce false
    (:Completed
      (Default|CallTargetDetected)
      (Utilities|FlowControl|DoOnce true) ; enters at Reset
    )))

(event EventHandleDirectorCommand
  (params (In%20Command :type S%20Director%20Command%20Structure))
  ;[0.2275 0.2275 0.2275] Mainly called by Director AI
  ; Prioritized over Patrol Mode
  ; Won't have any effect if called during an active chase
  (CallFunction|HandleCommand In%20Command))

(event EventSetChaseMode
  (params (NewChaseMode :type E_ChaserMode%20Enum :default "NewEnumerator0"))
  ;[0.2275 0.2275 0.2275] Mainly called by Service Nodes in the ChaserMaster BT
  (CallFunction|ToggleKillZone NewChaseMode)
  (CallFunction|ToggleMaxWalkSpeed NewChaseMode)
  (switch Utilities|FlowControl|Switch|SwitchonE_ChaserMode NewChaseMode
    (:NewEnumerator0
      (CallFunction|NotifyTargetLost))
    (:NewEnumerator1
      (CallFunction|NotifyTargetDetected))))

(event EventToggleScatter
  (params (IsActive? :type Boolean))
  ;[0.2275 0.2275 0.2275] -Toggle Scatter Mode
  ; -Clear Target if Scatter is activated (mainly relevant for revenant)
  (CallFunction|SetScatterMode IsActive?)
  (if IsActive?
    (CallFunction|ClearCurrentTarget)))

(event EventNotifyTargetLost
  ;[0.2275 0.2275 0.2275] Called when Chaser Mode changes. Do Once Gates to keep the ActiveChase counter in check
  (Utilities|FlowControl|DoOnce true
    (:Completed
      (Default|CallTargetLost)
      (Utilities|FlowControl|DoOnce false) ; enters at Reset
    )))

(event EventBeginPlay
  ;[0.2275 0.2275 0.2275] Required so that Ghosts don't start off which 500m/s max walk speed
  (CallFunction|SetChaseMode "NewEnumerator0"))

(fn ConstructionScript)

(fn ToggleKillZone
  (params (NewChaseMode :type E_ChaserMode%20Enum :default "NewEnumerator0"))
  (Variables|/Script/Engine.PrimitiveComponent|SetbGenerateOverlapEvents (Variables|Default|GetKillZone) (Utilities|Select :Index NewChaseMode :NewEnumerator0 false :NewEnumerator1 true :NewEnumerator2 true :NewEnumerator3 true)))

(fn ToggleMaxWalkSpeed
  (params (NewChaseMode :type E_ChaserMode%20Enum :default "NewEnumerator0"))
  (bind _chasespeed (Variables|Behavior|GetChaseSpeed))
  (Variables|/Script/Engine.CharacterMovementComponent|SetMaxWalkSpeed (Variables|Character|GetCharacterMovement) (Utilities|Select :Index NewChaseMode :NewEnumerator0 (Variables|Behavior|GetSearchSpeed) :NewEnumerator1 _chasespeed :NewEnumerator2 _chasespeed :NewEnumerator3 _chasespeed)))

(fn TryKillNearby
  (params (OverlappedActor :type Actor%20Object%20Reference))
  (bind _returnvalue (Utilities|DoesObjectImplementInterface OverlappedActor "/Game/Blueprints/Interfaces/I_Killable.I_Killable_C"))
  (if _returnvalue
    (Class|IKillable|Die(Message) OverlappedActor)
    (return _returnvalue)))

(fn SetScatterMode
  (params (Active? :type Boolean))
  (AI|Components|Blackboard|SetValueasBool (AI|GetBlackboard (Pawn|GetController)) (CallFunction|GetChaserBBKey "NewEnumerator2") Active?))

(fn BindtoChaserDirector
  (params (DirectorRef :type BP%20Chaser%20Director%20Object%20Reference))
  (EventDispatchers|BindEventtoTargetLost (EventDispatchers|CreateEvent DirectorRef :!event EventonChaserLostTarget))
  (EventDispatchers|BindEventtoTargetDetected (EventDispatchers|CreateEvent DirectorRef :!event EventonChaserDetectedTarget)))

(fn SetCommandLocation
  (params (VectorValue :type Vector) (Priority :type E_CommandPriority%20Enum :default "NewEnumerator0"))
  (bind _returnvalue (Pawn|GetController))
  (bind _returnvalue_2 (AI|GetBlackboard _returnvalue))
  (switch Utilities|FlowControl|Switch|SwitchonE_CommandPriority Priority
    (:NewEnumerator0
      (AI|Components|Blackboard|SetValueasVector _returnvalue_2 (CallFunction|GetChaserBBKey "NewEnumerator5") VectorValue :!label _label))
    (:NewEnumerator1
      (AI|Components|Blackboard|SetValueasVector _returnvalue_2 (CallFunction|GetChaserBBKey "NewEnumerator6") VectorValue))
    (:NewEnumerator2
      (goto _label))))

(fn ClearCurrentTarget
  (AI|Components|Blackboard|ClearValue (AI|GetBlackboard (Pawn|GetController)) (CallFunction|GetChaserBBKey "NewEnumerator0")))

(fn HandleCommand
  (params (In%20Command :type S%20Director%20Command%20Structure%20%28by%20ref%29))
  (bind (_commandtype _priority _targetlocation _targetactor _scatterstate) (Utilities|Struct|BreakS_DirectorCommand In%20Command))
  (switch Utilities|FlowControl|Switch|SwitchonE_CommandType _commandtype
    (:NewEnumerator0
      (CallFunction|SetCommandLocation _targetlocation _priority))
    (:NewEnumerator1
      (CallFunction|SetCommandLocation (Transformation|GetActorLocation _targetactor) _priority))
    (:NewEnumerator2
      (CallFunction|ToggleScatter _scatterstate))))

(fn GetChaseDuration
  (return (Variables|Behavior|GetChaseDuration)))

(fn GetChaserType
  (return (Variables|Behavior|GetBehavior)))

(fn GetCloseDistance
  (return (Variables|Behavior|GetCloseDistance)))

(fn GetScatterLocation
  (bind _scattercorner (Variables|Default|GetScatterCorner)
    (:then
      (return (Transformation|GetActorLocation _scattercorner)))
    (:else
      (return (Transformation|GetActorLocation)))))