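; AI controller for chaser enemies that hunt the player, each chaser type using its own chase style.
; It runs a master behavior tree and injects a direct, intercept, co-direct or shy chase subtree by gameplay tag, based on the pawn's reported type.
; It also copies the pawn's scatter location into the blackboard.
; AI perception sets the blackboard target when the player is sensed and clears it when forgotten.
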(event OnTargetPerceptionForgotten(AIPerception)
  (params (Actor :type Actor%20Object%20Reference))
  (CallFunction|HandlePerceptionForgetActor Actor))

(event OnTargetPerceptionUpdated(AIPerception)
  (params (Actor :type Actor%20Object%20Reference) (Stimulus :type AI%20Stimulus%20Structure))
  (CallFunction|HandlePerceptionUpdate Actor Stimulus))

(event Custom|Event%20RunNewBehavior
  (params (New%20Behavior :type Behavior%20Tree%20Object%20Reference))
  (AI|RunBehaviorTree New%20Behavior))

(event EventBeginPlay
  (AI|RunBehaviorTree "/Game/Blueprints/Enemy/AI/BehaviorTrees/BT_ChaserMaster.BT_ChaserMaster")
  (CallFunction|InitializeChaseBehavior)
  (CallFunction|InitializeScatterLocation))

(fn ConstructionScript)

(fn InitializeChaseBehavior
  (bind _asbehavior_tree_component (Utilities|Casting|CastToBehaviorTreeComponent (Variables|Default|GetBrainComponent)))
  (bind _out_type (Class|BPIChaser|GetChaserType(Message) (Pawn|GetControlledPawn)))
  (switch Utilities|FlowControl|Switch|SwitchonE_ChaserType _out_type
    (:NewEnumerator0
      (Class|BehaviorTreeComponent|SetDynamicSubtree _asbehavior_tree_component "(TagName=\"AI.Behavior.Chase\")" "/Game/Blueprints/Enemy/AI/BehaviorTrees/BT_DirectChase.BT_DirectChase"))
    (:NewEnumerator1
      (Class|BehaviorTreeComponent|SetDynamicSubtree _asbehavior_tree_component "(TagName=\"AI.Behavior.Chase\")" "/Game/Blueprints/Enemy/AI/BehaviorTrees/BT_InterceptChase.BT_InterceptChase"))
    (:NewEnumerator2
      (Class|BehaviorTreeComponent|SetDynamicSubtree _asbehavior_tree_component "(TagName=\"AI.Behavior.Chase\")" "/Game/Blueprints/Enemy/AI/BehaviorTrees/BT_CoDirectChase.BT_CoDirectChase"))
    (:NewEnumerator3
      (Class|BehaviorTreeComponent|SetDynamicSubtree _asbehavior_tree_component "(TagName=\"AI.Behavior.Chase\")" "/Game/Blueprints/Enemy/AI/BehaviorTrees/BT_ShyChase.BT_ShyChase"))))

(fn HandlePerceptionUpdate
  (params (PerceivedActor :type Actor%20Object%20Reference) (Stimulus :type AI%20Stimulus%20Structure%20%28by%20ref%29))
  ;[1 1 1] If Player is seen, set it as TargetActor to chase
  (if (Utilities|Struct|BreakAIStimulus Stimulus)
    ;;[0.1146 0.1146 0.1146] Cycle through tags to check if perceived actor is the player
    (bind _array_element (Utilities|Array|ForEachLoopwithBreak (Variables|/Script/Engine.Actor|GetTags PerceivedActor) :!label _label)
      (:LoopBody
        (switch name _array_element
          (:Player
            (AI|Components|Blackboard|SetValueasObject (AI|GetBlackboard 0) (CallFunction|GetChaserBBKey "NewEnumerator0") PerceivedActor)
            (Development|PrintString "Player spotted!" true true "(R=1.000000,G=0.502892,B=0.000000,A=1.000000)")
            (goto _label Break)))))))

(fn HandlePerceptionForgetActor
  (params (ForgottenActor :type Actor%20Object%20Reference))
  ;[1 1 1] If forgotten actor is player - clear TargetActor value from Blackboard
  (for _array_element (Variables|/Script/Engine.Actor|GetTags ForgottenActor)
    (switch name _array_element
      (:Player
        (AI|Components|Blackboard|ClearValue (AI|GetBlackboard 0) (CallFunction|GetChaserBBKey "NewEnumerator0"))
        (Development|PrintString "Forgot Player" true true "(R=0.045263,G=1.000000,B=0.000000,A=1.000000)")))))

(fn InitializeScatterLocation
  (bind _location (Class|BPIChaser|GetScatterLocation(Message) (Pawn|GetControlledPawn)))
  (AI|Components|Blackboard|SetValueasVector (AI|GetBlackboard 0) (CallFunction|GetChaserBBKey "NewEnumerator3") _location))