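; AI controller for ghost chaser enemies that pursue the player using a shared master behavior tree.
; It injects a chase subtree matching the pawn's chaser type (direct, intercept, co-direct, shy, runner or stalker) via a gameplay tag.
; Perception sets the blackboard target unless the ghost is scattering, and clears it when forgotten.
; The pawn also supplies the scatter location and chase duration, the latter applied as sight sense max age.
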(event OnTargetPerceptionForgotten(AIPerception)
  (params (Actor :type Actor%20Object%20Reference))
  (CallFunction|HandlePerceptionForgetActor Actor))

(event OnTargetPerceptionUpdated(AIPerception)
  (params (Actor :type Actor%20Object%20Reference) (Stimulus :type AI%20Stimulus%20Structure))
  (CallFunction|HandlePerceptionUpdate Actor Stimulus))

(event Custom|Event%20RunNewBehavior
  (params (New%20Behavior :type Behavior%20Tree%20Object%20Reference))
  (AI|RunBehaviorTree New%20Behavior))

(event EventBeginPlay
  (AI|RunBehaviorTree "/Game/Blueprints/Enemy/DirectorControlled/AI/BehaviorTrees/BT_ChaserMaster.BT_ChaserMaster")
  (CallFunction|InitializeChaseBehavior)
  (CallFunction|InitializeScatterLocation)
  (Utilities|FlowControl|DelayUntilNextTick)
  (CallFunction|InitializeChaseDuration))

(event EventPossess
  (params (PossessedPawn :type Pawn%20Object%20Reference))
  (CallFunction|InitializeChaseBehavior))

(fn ConstructionScript)

(fn InitializeChaseBehavior
  (bind _asbehavior_tree_component (Utilities|Casting|CastToBehaviorTreeComponent (Variables|Default|GetBrainComponent)))
  (bind _out_type (Class|BPIDirectorChaser|GetChaserType(Message) (Pawn|GetControlledPawn)))
  (switch Utilities|FlowControl|Switch|SwitchonE_ChaserType _out_type
    (:NewEnumerator0
      (Class|BehaviorTreeComponent|SetDynamicSubtree _asbehavior_tree_component "(TagName=\"AI.Behavior.Chase\")" "/Game/Blueprints/Enemy/DirectorControlled/AI/BehaviorTrees/BT_DirectChase.BT_DirectChase"))
    (:NewEnumerator1
      (Class|BehaviorTreeComponent|SetDynamicSubtree _asbehavior_tree_component "(TagName=\"AI.Behavior.Chase\")" "/Game/Blueprints/Enemy/DirectorControlled/AI/BehaviorTrees/BT_InterceptChase.BT_InterceptChase"))
    (:NewEnumerator2
      (Class|BehaviorTreeComponent|SetDynamicSubtree _asbehavior_tree_component "(TagName=\"AI.Behavior.Chase\")" "/Game/Blueprints/Enemy/DirectorControlled/AI/BehaviorTrees/BT_CoDirectChase.BT_CoDirectChase"))
    (:NewEnumerator3
      (Class|BehaviorTreeComponent|SetDynamicSubtree _asbehavior_tree_component "(TagName=\"AI.Behavior.Chase\")" "/Game/Blueprints/Enemy/DirectorControlled/AI/BehaviorTrees/BT_ShyChase.BT_ShyChase"))
    (:NewEnumerator5
      (Class|BehaviorTreeComponent|SetDynamicSubtree _asbehavior_tree_component "(TagName=\"AI.Behavior.Chase\")" "/Game/Blueprints/Enemy/DirectorControlled/AI/BehaviorTrees/BT_Sub_Scatter.BT_Sub_Scatter"))
    (:NewEnumerator6
      (Class|BehaviorTreeComponent|SetDynamicSubtree _asbehavior_tree_component "(TagName=\"AI.Behavior.Chase\")" "/Game/Blueprints/Enemy/DirectorControlled/AI/BehaviorTrees/BT_Stalker.BT_Stalker"))))

(fn HandlePerceptionUpdate
  (params (PerceivedActor :type Actor%20Object%20Reference) (Stimulus :type AI%20Stimulus%20Structure%20%28by%20ref%29))
  ;[1 1 1] If Player is seen, set it as TargetActor to chase
  (if (Utilities|Struct|BreakAIStimulus Stimulus)
    ;;[0.1146 0.1146 0.1146] Cycle through tags to check if perceived actor is the player
    (bind _array_element (Utilities|Array|ForEachLoopwithBreak (Variables|/Script/Engine.Actor|GetTags PerceivedActor) :!label _label)
      (:LoopBody
        (switch name _array_element
          (:Player
            (if (not (ScalableFloat|GetValueasBool (AI|GetBlackboard 0) (CallFunction|GetChaserBBKey "NewEnumerator2")))
              (AI|Components|Blackboard|SetValueasObject (AI|GetBlackboard 0) (CallFunction|GetChaserBBKey "NewEnumerator0") PerceivedActor)
              (Development|PrintString "Player spotted!" true true "(R=1.000000,G=0.502892,B=0.000000,A=1.000000)")
              (goto _label Break))))))))

(fn HandlePerceptionForgetActor
  (params (ForgottenActor :type Actor%20Object%20Reference))
  (bind _keyout (CallFunction|GetChaserBBKey "NewEnumerator0"))
  (bind _returnvalue (AI|GetBlackboard 0))
  ;[1 1 1] If forgotten actor is current TargetActor - clear TargetActor value from Blackboard
  (if (== ForgottenActor (AI|Components|Blackboard|GetValueasObject _returnvalue _keyout))
    (AI|Components|Blackboard|ClearValue _returnvalue _keyout)
    (Development|PrintString "Forgot Player" true true "(R=0.045263,G=1.000000,B=0.000000,A=1.000000)")))

(fn InitializeScatterLocation
  (bind _location (Class|BPIDirectorChaser|GetScatterLocation(Message) (Pawn|GetControlledPawn)))
  (AI|Components|Blackboard|SetValueasVector (AI|GetBlackboard 0) (CallFunction|GetChaserBBKey "NewEnumerator3") _location))

(fn InitializeChaseDuration
  (bind _duration (Class|BPIDirectorChaser|GetChaseDuration(Message) (Pawn|GetControlledPawn)))
  (Class|AIPerceptionUtils|SetSightSenseMaxAge self _duration))