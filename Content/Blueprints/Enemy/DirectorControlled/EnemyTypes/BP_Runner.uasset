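; BP_Runner is a director-controlled enemy type that sets up a scatter destination when notified that a target is detected.
; On that notification it runs the parent logic, then stores a random BP_ZoneCorner from the level as its ScatterCorner.
; It then tells its BP_ChaseAIController to initialize the scatter location.
; All other behavior comes from the parent class.
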(event EventBeginPlay
  (|CallParentFunction) ; This node is disabled and will not be called.\nDrag off pins to build functionality.
)

(event Collision|EventActorBeginOverlap
  (params (OtherActor :type Actor%20Object%20Reference)))

(event EventTick
  (params (DeltaSeconds :type Float%20%28single-precision%29)))

(event EventNotifyTargetDetected
  (|CallParentFunction)
  (bind _outactors (Actor|GetAllActorsOfClass "/Game/Blueprints/Zones/BP_ZoneCorner.BP_ZoneCorner_C"))
  (Variables|Default|SetScatterCorner (.OutItem (Utilities|Array|Random _outactors)))
  (bind _asbp_chase_aicontroller (Utilities|Casting|CastToBP_ChaseAIController (AI|GetAIController self)))
  (Default|InitializeScatterLocation _asbp_chase_aicontroller))

(fn ConstructionScript
  (|CallParentFunction))