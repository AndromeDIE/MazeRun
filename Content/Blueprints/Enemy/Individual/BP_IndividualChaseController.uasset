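; AI controller for individual chasing enemies that detects and tracks the player.
; On BeginPlay it runs the BT_IndividualEnemyMaster behavior tree.
; When AI perception senses an actor tagged Player, it writes that actor to an enum-derived blackboard key.
; The key is cleared only when perception forgets that same actor, so losing sight alone keeps the target.
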(event OnTargetPerceptionUpdated(AIPerception)
  (params (Actor :type Actor%20Object%20Reference) (Stimulus :type AI%20Stimulus%20Structure))
  (if (and (Actor|ActorHasTag Actor "Player") (Utilities|Struct|BreakAIStimulus Stimulus))
    (AI|Components|Blackboard|SetValueasObject (AI|GetBlackboard 0) (CallFunction|GetChaserBBKey "NewEnumerator0") Actor)))

(event OnTargetPerceptionForgotten(AIPerception)
  (params (Actor :type Actor%20Object%20Reference))
  (bind _keyout (CallFunction|GetChaserBBKey "NewEnumerator0"))
  (bind _returnvalue (AI|GetBlackboard 0))
  (if (== Actor (AI|Components|Blackboard|GetValueasObject _returnvalue _keyout))
    (AI|Components|Blackboard|ClearValue _returnvalue _keyout)))

(event EventBeginPlay
  (AI|RunBehaviorTree "/Game/Blueprints/Enemy/Individual/AI/BT_IndividualEnemyMaster.BT_IndividualEnemyMaster"))

(fn ConstructionScript)