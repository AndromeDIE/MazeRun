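; Enemy component that gives an individual a memory of target orbs it has spotted and detects when a known orb has been picked up.
; Spotted orbs are stored in a state map with a forget timer that counts down on Tick; expired orbs change state and are notified.
; Seeing a known orb picked up marks it collected once and fires an event.
; It can also return a random unexplored orb from memory.
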(event Custom|Event%20OnOwnerSpottedOrb
  (params (SpottedOrb :type Actor%20Object%20Reference))
  (bind _asbp_target_orb (Utilities|Casting|CastToBP_TargetOrb SpottedOrb))
  (if (Variables|/Game/Blueprints/GameObjects/Pickups/BP_TargetOrb.BP_TargetOrb_C|GetPickedUp? _asbp_target_orb)
    (CallFunction|HandleStimulusonPickedUpOrb _asbp_target_orb)
    (else
      (CallFunction|AddOrbtoMemory _asbp_target_orb))))

(event Custom|Event%20AddNewOrbTimer
  (params (OrbRef :type Actor%20Object%20Reference) (ForgetTime :type Float%20%28double-precision%29))
  (Utilities|Map|Add (Variables|Default|GetOrbForgetTimer) OrbRef ForgetTime)
  (Development|PrintString "Added Orb forget timer" true true "(R=0.000000,G=0.660000,B=1.000000,A=1.000000)" 2.0 "AddOrbForgetTimer")
  (Class|IIndividualMemorizable|OnIndividualSeen(Message) OrbRef))

(event Custom|Event%20ForgetOrb
  (params (OrbRef :type Actor%20Object%20Reference))
  (CallFunction|RemoveOrbfromTimerMap OrbRef)
  (Utilities|IsValid OrbRef
    (:Is%20Valid
      (Utilities|Map|Add (Variables|Default|GetOrbMap) OrbRef "NewEnumerator0")
      (Class|IIndividualMemorizable|OnIndividualForgot(Message) OrbRef)
      (Development|PrintString "Forgot Orb" true true (Math|Color|MakeColor (Math|Random|RandomFloat) (Math|Random|RandomFloat) (Math|Random|RandomFloat) (Math|Random|RandomFloat)) 2.0 "ForgotOrb"))))

(event Custom|Event%20OnKnownOrbPickedUp
  (params (PickupLocation :type Vector) (OrbRef :type BP%20Base%20Pickup%20Object%20Reference))
  (Utilities|FlowControl|Sequence
    (:then_0
      (CallFunction|RemoveOrbfromTimerMap OrbRef)
      (Utilities|Map|Add (Variables|Default|GetOrbMap) OrbRef "NewEnumerator2")
      (Default|CallOnKnownOrbCollected))
    (:then_1
      (Development|PrintString "KNOWN ORB COLLECTED" true true "(R=1.000000,G=0.025124,B=0.000000,A=1.000000)" 2.0 "ORBWARNING"))))

(event EventTick
  (params (DeltaSeconds :type Float%20%28single-precision%29))
  (if (not (Utilities|Map|IsEmpty (Variables|Default|GetOrbForgetTimer)))
    (CallFunction|UpdateForgetTimers DeltaSeconds)))

(fn UpdateForgetTimers
  (params (DeltaTime :type Float%20%28single-precision%29))
  (bind _orbstoforget (LocalVariables|GetOrbsToForget))
  (bind _orbforgettimer (Variables|Default|GetOrbForgetTimer))
  (Utilities|FlowControl|Sequence
    (:then_0
      (bind _keys (Utilities|Map|Keys (Variables|Default|GetOrbForgetTimer)))
      (for _array_element _keys
        (if (.ReturnValue (Utilities|Map|Find _orbforgettimer _array_element))
          (Utilities|Map|Add _orbforgettimer _array_element (- (.Value (Utilities|Map|Find _orbforgettimer _array_element)) DeltaTime)))))
    (:then_1
      (bind _keys_2 (Utilities|Map|Keys (Variables|Default|GetOrbForgetTimer)))
      (for _array_element_2 _keys_2
        (if (<= (.Value (Utilities|Map|Find (Variables|Default|GetOrbForgetTimer) _array_element_2)) 0.0)
          (Utilities|Array|Add (LocalVariables|GetOrbsToForget) _array_element_2))))
    (:then_2
      (for _array_element_3 _orbstoforget
        (CallFunction|EventForgetOrb _array_element_3))
      (Utilities|Array|Clear _orbstoforget)
      (Development|PrintString (Utilities|String|ToString(Integer) (Utilities|Map|Length (Variables|Default|GetOrbForgetTimer))) true true "(R=1.000000,G=0.027728,B=0.756932,A=1.000000)" 2.0 "KnownOrbs")
      (Development|PrintString (Utilities|String|ToString(Integer) (Utilities|Map|Length (Variables|Default|GetOrbMap))) true true "(R=0.981706,G=1.000000,B=0.000000,A=1.000000)" 2.0 "KnownOrbsSeen"))))

(fn AddOrbtoMemory
  (params (OrbToAdd :type Actor%20Object%20Reference))
  (Utilities|Map|Add (Variables|Default|GetOrbMap) OrbToAdd "NewEnumerator1")
  (CallFunction|EventAddNewOrbTimer OrbToAdd (Variables|Default|GetOrbForgetTime)))

(fn RemoveOrbfromTimerMap
  (params (OrbToRemove :type Actor%20Object%20Reference%20%28by%20ref%29))
  (Utilities|Map|Remove (Variables|Default|GetOrbForgetTimer) OrbToRemove))

(fn GetRandomUnexploredOrb
  (bind _orbmap (Variables|Default|GetOrbMap))
  (bind _unexploredorbs (LocalVariables|GetUnexploredOrbs))
  (Utilities|FlowControl|Sequence
    (:then_0
      (bind _keys (Utilities|Map|Keys _orbmap))
      (for _array_element _keys
        (if (Utilities|Enum|Equal(Enum) (.Value (Utilities|Map|Find _orbmap _array_element)) "NewEnumerator0")
          (Utilities|Array|Add (LocalVariables|GetUnexploredOrbs) _array_element))))
    (:then_1
      (if (not (Utilities|Array|IsEmpty _unexploredorbs))
        (return (.OutItem (Utilities|Array|Random _unexploredorbs)))))))

(fn HandleStimulusonPickedUpOrb
  (params (OrbRef :type BP%20Target%20Orb%20Object%20Reference))
  (bind _orbmap (Variables|Default|GetOrbMap))
  (bind (_value _returnvalue) (Utilities|Map|Find _orbmap OrbRef))
  ;[1 1 1] Call Event only if the Orb was known before and hasn't already been discovered missing
  (if (not (or (Utilities|Enum|Equal(Enum) _value "NewEnumerator2") (not _returnvalue)))
    (CallFunction|EventonKnownOrbPickedUp (Transformation|GetActorLocation OrbRef) OrbRef)))