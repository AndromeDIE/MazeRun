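; BP_BasePickup is a base pickup actor that handles being collected in the game.
; Its PickUp event fires the PickedUp dispatcher with the pickup's location and a self reference, then plays feedback and destroys the actor.
; Sound and particle effects come from helper functions that spawn PickupSound and a scaled PickupVFX emitter at the actor's location.
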(event EventPickUp
  (Default|CallPickedUp (Transformation|GetActorLocation) self)
  (CallFunction|PlayPickupSound)
  (CallFunction|PlayPickupVFX)
  (Actor|DestroyActor))

(fn ConstructionScript)

(fn PlayPickupSound
  (Audio|PlaySoundatLocation (Variables|Default|GetPickupSound) (Transformation|GetActorLocation) "0, 0, 0" 1.0 1.0 0.0 0 0 0 0))

(fn PlayPickupVFX
  (Effects|SpawnEmitteratLocation (Variables|Default|GetPickupVFX) (Transformation|GetActorLocation) "0, 0, 0" (Variables|Default|GetPickupVFX_Scale)))