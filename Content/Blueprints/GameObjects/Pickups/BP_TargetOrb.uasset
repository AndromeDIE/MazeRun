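; BP_TargetOrb is a pickup orb that shows whether an individual has forgotten, seen or is checking it.
; Each state event swaps the sphere material, and the check state also lights WarnLight and starts a timer that reverts to forgotten.
; Seen and forgotten clear that timer and turn the light off.
; PickUp broadcasts location and self, plays sound and VFX, then disables overlaps and hides the sphere.
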(event EventOnIndividualForgot
  (Rendering|Material|SetMaterial (Variables|Default|GetSphere) 0 "/Game/Materials/M_Unexplored.M_Unexplored")
  (Utilities|Time|ClearandInvalidateTimerbyHandle (stale EventOnIndividualCheck _returnvalue))
  (Rendering|Components|Light|SetIntensity (Variables|Default|GetWarnLight) 0.0))

(event EventOnIndividualSeen
  (Rendering|Material|SetMaterial (Variables|Default|GetSphere) 0 "/Game/Materials/M_ShyChaser.M_ShyChaser")
  (Utilities|Time|ClearandInvalidateTimerbyHandle (stale EventOnIndividualCheck _returnvalue))
  (Rendering|Components|Light|SetIntensity (Variables|Default|GetWarnLight) 0.0))

(event EventOnIndividualCheck
  (Rendering|Material|SetMaterial (Variables|Default|GetSphere) 0 "/Game/Materials/M_DirectChaser.M_DirectChaser")
  (Rendering|Components|Light|SetIntensity (Variables|Default|GetWarnLight) (Variables|Default|GetWarnLightIntensity))
  (bind _returnvalue (Utilities|Time|SetTimerbyEvent (delegate EventOnIndividualForgot) 1e+01)))

(event EventPickUp
  (Default|CallPickedUp (Transformation|GetActorLocation) self)
  (CallFunction|PlayPickupSound)
  (CallFunction|PlayPickupVFX)
  (Variables|Default|SetPickedUp? true)
  (Variables|/Script/Engine.PrimitiveComponent|SetbGenerateOverlapEvents (Variables|Default|GetPickupZone) false)
  (Variables|/Script/Engine.PrimitiveComponent|SetbGenerateOverlapEvents (Variables|Default|GetSphere) false)
  (Rendering|SetVisibility (Variables|Default|GetSphere) false false))

(fn ConstructionScript)